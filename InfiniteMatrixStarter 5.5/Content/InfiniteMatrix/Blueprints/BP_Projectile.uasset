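; BP_Projectile is a projectile that reacts to whatever its sphere collider begins overlapping.
; A cast chain identifies the hit: a HealthPack or Enemy is destroyed along with the projectile, after the stored Player reference processes the pickup or takedown.
; Hitting a BP_Tunnel destroys only the projectile, and all other overlaps are ignored.
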(event `self.Sphere.OnComponentBeginOverlap`
  (params (OverlappedComponent :type "PrimitiveComponent Object Reference") (OtherActor :type "Actor Object Reference") (OtherComp :type "PrimitiveComponent Object Reference") (OtherBodyIndex :type Integer) (bFromSweep :type Boolean) (SweepResult :type "HitResult Structure (by ref)"))
  (bind _player (`self.player`))
  (bind _ashealth_pack (cast `/Game/InfiniteMatrix/Blueprints/HealthPack` OtherActor)
    (:`then`
      (`/Game/InfiniteMatrix/Blueprints/BP_Player.Process Healthpack` _player)
      (`self.K2_DestroyActor` _ashealth_pack)
      (`self.K2_DestroyActor`))
    (:`CastFailed`
      (bind _asenemy (cast `/Game/InfiniteMatrix/Blueprints/Enemy` OtherActor)
        (:`then`
          (`/Game/InfiniteMatrix/Blueprints/BP_Player.Process Enemy Takedown` _player)
          (`self.K2_DestroyActor` _asenemy)
          (`self.K2_DestroyActor`))
        (:`CastFailed`
          (cast `/Game/InfiniteMatrix/Blueprints/BP_Tunnel` OtherActor)
          (`self.K2_DestroyActor`))))))

(fn `UserConstructionScript`)